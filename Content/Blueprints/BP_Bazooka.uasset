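; BP_Bazooka is a launcher actor whose Shoot function fires a rocket projectile.
; Shoot spawns the Projectile class at ProjectileSpawn, matches it to the root's rotation, then casts it to BP_Rocket.
; A velocity-change impulse scaled by ShootStrength pushes the rocket's Cube along Cube1's forward vector.
; The overlap trigger for BP_Hammond is disconnected, so nothing in this graph calls Shoot.
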(event EventBeginPlay)

(event EventTick
  (params (DeltaSeconds :type Float%20%28single-precision%29)))

(event Collision|EventActorBeginOverlap
  (params (OtherActor :type Actor%20Object%20Reference)))

(fn ConstructionScript)

(fn Shoot
  (bind _returnvalue (Game|SpawnActorfromClass (Variables|Default|GetProjectile) (Math|Conversions|ToTransform(Vector) (Transformation|GetWorldLocation (Variables|Default|GetProjectileSpawn))) "AdjustIfPossibleButAlwaysSpawn" 0 0))
  (Transformation|SetActorRotation _returnvalue (Transformation|GetWorldRotation (Variables|Default|GetDefaultSceneRoot)))
  (bind _asbp_rocket (Utilities|Casting|CastToBP_Rocket _returnvalue))
  (Physics|AddImpulse (Variables|/Game/Blueprints/BP_Rocket.BP_Rocket_C|GetCube _asbp_rocket) (* (Math|Vector|GetForwardVector (Variables|Default|GetCube1)) (Variables|Default|GetShootStrength)) "None" true))