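; Hammond is a player-controlled physics ball that rolls around and fires a bazooka.
; Camera-relative input spins the mesh up to a speed cap and adds velocity when a sphere trace finds no ground.
; Each tick the actor snaps to the simulated mesh, while spring arm, weapon ring and spawned bazooka follow control rotation.
; A scaled mesh serves as the health bar, and zero health reloads the level.
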(event EventBeginPlay
  ;[1 1 1] Bazooka go pow
  (bind _returnvalue (Game|SpawnActorfromClass "/Game/Blueprints/BP_Bazooka.BP_Bazooka_C" (Transformation|GetWorldTransform (Variables|Default|GetWeaponLeft)) "Undefined" self 0))
  (Utilities|Array|Add (Variables|Default|GetBazookas) _returnvalue)
  (Transformation|AttachActorToActor _returnvalue self "None" "KeepWorld" "KeepWorld" "KeepWorld" false)
  (Variables|Default|SetHealthPoints (Variables|Default|GetHealth)))

(event EventTick
  (params (DeltaSeconds :type Float%20%28single-precision%29))
  (if (> (Variables|Default|GetHealthPoints) 0)
    (Utilities|FlowControl|Sequence
      (:then_0
        (CallFunction|InAirMovement)
        (CallFunction|UpdateWeaponTransform)
        (CallFunction|RollBall)
        (CallFunction|HPBarUpdate))
      (:then_1
        (Transformation|SetWorldRotation (Variables|Default|GetSpringArm) (Pawn|GetControlRotation :!class /Script/Engine.Pawn) false false)
        (Transformation|SetActorLocation (Transformation|GetWorldLocation (Variables|Default|GetRollingBallMesh)) false false)))
    (else
      (bind _returnvalue (Game|GetCurrentLevelName true))
      (Game|OpenLevel(byName) (Utilities|String|StringToName _returnvalue)))))

(event Input|ActionEvents|InputActionShoot
  (params (Key :type Key%20Structure :default "None"))
  ;[1 1 1] Bazooka go pow
  (:Pressed
    (for _array_element (Variables|Default|GetBazookas)
      (Default|Shoot _array_element))))

(event Input|AxisEvents|InputAxisWalkRight
  (params (AxisValue :type Float%20%28single-precision%29))
  ;[1 1 1] Move input
  (Variables|Default|SetMoveDirectionR (* AxisValue (Math|Vector|GetRightVector (Math|Rotator|MakeRotator 0.0 0.0 (+ (.Yaw (Math|Rotator|BreakRotator (Pawn|GetControlRotation :!class /Script/Engine.Pawn))) 9e+01))))))

(event Input|AxisEvents|InputAxisWalkForward
  (params (AxisValue :type Float%20%28single-precision%29))
  ;[1 1 1] Move input
  (Variables|Default|SetMoveDirectionF (* (Math|Vector|GetForwardVector (Math|Rotator|MakeRotator 0.0 0.0 (+ (.Yaw (Math|Rotator|BreakRotator (Pawn|GetControlRotation :!class /Script/Engine.Pawn))) 9e+01))) AxisValue)))

(event Input|AxisEvents|InputAxisLookUp
  (params (AxisValue :type Float%20%28single-precision%29))
  ;[1 1 1] Look
  (Class|PlayerController|AddPitchInput (Game|GetPlayerController 0) (* (* AxisValue (Variables|Default|GetMouseSensitivity)) -1.0)))

(event Input|AxisEvents|InputAxisLookRight
  (params (AxisValue :type Float%20%28single-precision%29))
  ;[1 1 1] Look
  (Class|PlayerController|AddYawInput (Game|GetPlayerController 0) (* AxisValue (Variables|Default|GetMouseSensitivity))))

(fn ConstructionScript)

(fn InAirMovement
  (bind _collision (Variables|Default|GetCollision))
  (bind _returnvalue (Transformation|GetWorldLocation _collision))
  (bind _returnvalue_2 (Collision|SphereTraceForObjects _returnvalue (+ _returnvalue (Math|Vector|VectorDown)) (Components|Sphere|GetScaledSphereRadius _collision) (Utilities|Array|MakeArray "ObjectTypeQuery1" "ObjectTypeQuery2" "ObjectTypeQuery4") false 0 "None"))
  (if (not _returnvalue_2)
    (Physics|SetPhysicsLinearVelocity (Variables|Default|GetRollingBallMesh) (* (Math|Vector|RotateVectorAroundAxis (Math|Vector|Normalize (+ (Variables|Default|GetMoveDirectionR) (Variables|Default|GetMoveDirectionF))) -9e+01 "0, 0,1.000000") (* (Variables|Default|GetInAirMoveForce) (Utilities|Time|GetWorldDeltaSeconds))) true "None")))

(fn UpdateWeaponTransform
  (bind _returnvalue (Pawn|GetControlRotation :!class /Script/Engine.Pawn))
  (bind _bazookas (Variables|Default|GetBazookas))
  (bind _output (Utilities|Array|Get(acopy) _bazookas))
  (Transformation|SetWorldRotation (Variables|Default|GetWeaponRingMesh) (Math|Rotator|MakeRotator 0.0 9e+01 (.yaw _returnvalue)) false false)
  (Transformation|SetActorRelativeRotation _output (Math|Rotator|MakeRotator 0.0 (.pitch _returnvalue) (.yaw _returnvalue)))
  (Transformation|SetActorLocation _output (Transformation|GetWorldLocation (Variables|Default|GetWeaponLeft)) false false))

(fn RollBall
  (Class|PrimitiveComponent|SetAllPhysicsAngularVelocityinDegrees (Variables|Default|GetRollingBallMesh) (* (Math|Vector|Normalize (+ (Variables|Default|GetMoveDirectionR) (Variables|Default|GetMoveDirectionF))) (* (Variables|Default|GetRollAcceleration) (/ (Utilities|Time|GetWorldDeltaSeconds) (Variables|Default|GetRollAccelerationTime)))) true)
  (if (> (Math|Vector|VectorLength (Physics|GetPhysicsAngularVelocityinDegrees (Variables|Default|GetRollingBallMesh) "None")) (Variables|Default|GetMaxRollSpeed))
    (Class|PrimitiveComponent|SetAllPhysicsAngularVelocityinDegrees (Variables|Default|GetRollingBallMesh) (* (Math|Vector|Normalize (+ (Variables|Default|GetMoveDirectionR) (Variables|Default|GetMoveDirectionF))) (Variables|Default|GetMaxRollSpeed)) false)))

(fn HPBarUpdate
  (Transformation|SetWorldScale3D (Variables|Default|GetHPMesh) (Math|Vector|MakeVector 0.25 (/ (Variables|Default|GetHealthPoints) (Math|Conversions|ToFloat(Integer) (Variables|Default|GetHealth))) 0.25)))