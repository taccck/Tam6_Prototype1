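; BP_Rocket is a short-lived rocket projectile that explodes on impact and damages enemies or the Hammond player pawn.
; On hit it spawns an explosion effect with configurable radial impulse, subtracts health, then removes itself after a short delay.
; Airborne enemies take extra damage and count airshots, with repeat airshots raising sound pitch and revealing a second widget.
; Tick keeps both airshot widgets facing opposite the player camera's forward vector.
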(event OnComponentHit(StaticMesh)
  (params (HitComponent :type Primitive%20Component%20Object%20Reference) (OtherActor :type Actor%20Object%20Reference) (OtherComp :type Primitive%20Component%20Object%20Reference) (NormalImpulse :type Vector :default "0, 0, 0") (Hit :type Hit%20Result%20Structure%20%28by%20ref%29))
  (bind _returnvalue (Game|SpawnActorfromClass "/Game/StarterContent/Blueprints/Blueprint_Effect_Explosion.Blueprint_Effect_Explosion_C" (Math|Conversions|ToTransform(Vector) (Transformation|GetWorldLocation (Variables|Default|GetStaticMesh))) "Undefined" 0 0))
  (Variables|/Script/Engine.RadialForceComponent|SetImpulseStrength (Variables|/Game/StarterContent/Blueprints/Blueprint_Effect_Explosion.Blueprint_Effect_Explosion_C|GetRadialForce _returnvalue) (Variables|Default|GetExplosion%20strength))
  (bind _asbp_enemy (Utilities|Casting|CastToBP_Enemy OtherActor)
    (:then
      (Math|Integer|DecrementInt (Variables|/Game/Blueprints/BP_Enemy.BP_Enemy_C|GetHealthPoints _asbp_enemy)
        (:%20%20
          (if (Variables|/Game/Blueprints/BP_Enemy.BP_Enemy_C|GetOnground _asbp_enemy)
            (Audio|PlaySound2D (Variables|Default|GetHitEnemySound) 1.0 1.0 0.0 0 0)
            (else
              (bind _result (Math|Integer|IncrementInt (Variables|/Game/Blueprints/BP_Enemy.BP_Enemy_C|GetAirshots _asbp_enemy))
                (:%20%20
                  (Math|Integer|DecrementInt (Variables|/Game/Blueprints/BP_Enemy.BP_Enemy_C|GetHealthPoints _asbp_enemy)
                    (:%20%20
                      (if (> _result 1)
                        (Audio|PlaySound2D "/Game/SOUND/airshot.airshot" 1.0 1.5 0.0 0 0)
                        (Class|WidgetComponent|SetTintColorandOpacity (Variables|Default|Getairshotwidget2) "(R=1.000000,G=1.000000,B=1.000000,A=1.000000)")
                        (else
                          (Audio|PlaySound2D "/Game/SOUND/airshot.airshot" 1.0 1.0 0.0 0 0)
                          (Class|WidgetComponent|SetTintColorandOpacity (Variables|Default|Getairshotwidget) "(R=1.000000,G=1.000000,B=1.000000,A=1.000000)"))))))))))))
    (:CastFailed
      (bind _asbp_hammond (Utilities|Casting|CastToBP_Hammond OtherActor)
        (:then
          (Math|Integer|DecrementInt (Variables|/Game/Blueprints/BP_Hammond.BP_Hammond_C|GetHealthPoints _asbp_hammond)
            (:%20%20
              (Audio|PlaySound2D (Variables|Default|GetHitPlayerSound) 1.0 1.0 0.0 0 0))))
        (:CastFailed
          _))))
  (Components|DestroyComponent (Variables|Default|GetStaticMesh))
  (Utilities|FlowControl|Delay 0.5)
  (Actor|DestroyActor))

(event EventBeginPlay
  (Actor|SetLifeSpan 3.0))

(event EventTick
  (params (DeltaSeconds :type Float%20%28single-precision%29))
  (bind _asbp_hammond (Utilities|Casting|CastToBP_Hammond (Game|Player|GetPlayerPawn 0)))
  (Transformation|SetWorldRotation (Variables|Default|Getairshotwidget) (Math|Rotator|MakeRotfromX (Math|Vector|NegateVector (Math|Vector|GetForwardVector (Variables|/Game/Blueprints/BP_Hammond.BP_Hammond_C|GetCamera _asbp_hammond)))) false false))

(fn ConstructionScript)