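; Rolling-ball enemy that chases the player and fires a bazooka spawned on its weapon ring at random moments.
; Each tick it estimates player movement from the position change, then uses that to steer the physics ball's capped spin and its airborne velocity nudge.
; The actor follows the ball's location, while ring and bazooka aim with a lead multiplier re-randomized at each shot.
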(event Custom|GetPlayerDirection
  (bind _collision (Variables|Default|GetCollision))
  (bind _playerref (Variables|Default|GetPlayerRef))
  (bind _playersvelocity (Variables|Default|GetPlayersVelocity))
  (bind _returnvalue (Transformation|GetWorldLocation _collision))
  (bind _collision_2 (Variables|/Game/Blueprints/BP_Hammond.BP_Hammond_C|GetCollision _playerref))
  (bind _returnvalue_2 (Transformation|GetWorldLocation _collision_2))
  (bind _returnvalue_3 (+ _returnvalue_2 _playersvelocity))
  ;[1 1 1] Look
  (Variables|Default|SetDirectionToPlayer (* (Math|Vector|Normalize (- _returnvalue_3 _returnvalue)) (/ (Math|Vector|Distance(Vector) _returnvalue _returnvalue_3) 1e+04))))

(event Custom|EnemyShoot
  ;[1 1 1] Bazooka go pow
  (for _array_element (Variables|Default|GetBazookas)
    (Variables|Default|SetVelocityOffset (Math|Random|RandomFloatinRange (Variables|Default|GetVelocityMin) (Variables|Default|GetCwlocityMax)))
    (Default|Shoot _array_element)))

(event Custom|PlayerVelocity
  (bind _playerref (Variables|Default|GetPlayerRef))
  (bind _collision (Variables|/Game/Blueprints/BP_Hammond.BP_Hammond_C|GetCollision _playerref))
  (bind _returnvalue (Transformation|GetWorldLocation _collision))
  (Variables|Default|SetPlayersVelocity (- _returnvalue (Variables|Default|GetPlayersOldLocation)))
  (Variables|Default|SetPlayersOldLocation _returnvalue))

(event EventBeginPlay
  ;[1 1 1] Bazooka go pow
  (bind _returnvalue (Game|SpawnActorfromClass "/Game/Blueprints/BP_Bazooka.BP_Bazooka_C" (Transformation|GetWorldTransform (Variables|Default|GetWeaponLeft)) "Undefined" self 0))
  (Utilities|Array|Add (Variables|Default|GetBazookas) _returnvalue)
  (Transformation|AttachActorToActor _returnvalue self "None" "KeepWorld" "KeepWorld" "KeepWorld" false))

(event EventTick
  (params (DeltaSeconds :type Float%20%28single-precision%29))
  (CallFunction|PlayerVelocity)
  (CallFunction|GetPlayerDirection)
  (Utilities|FlowControl|Sequence
    (:then_0
      (CallFunction|InAirMovement)
      (CallFunction|UpdateWeaponTransform)
      (CallFunction|RollBall))
    (:then_1
      (Transformation|SetWorldRotation (Variables|Default|GetSpringArm) (Pawn|GetControlRotation :!class /Script/Engine.Pawn) false false)
      (Transformation|SetActorLocation (Transformation|GetWorldLocation (Variables|Default|GetRollingBallMesh)) false false)
      (if (== (Math|Random|RandomInteger 100) 0)
        (CallFunction|EnemyShoot)))))

(fn ConstructionScript)

(fn InAirMovement
  (bind _collision (Variables|Default|GetCollision))
  (bind _returnvalue (Transformation|GetWorldLocation _collision))
  (bind _returnvalue_2 (Collision|SphereTraceForObjects _returnvalue (+ _returnvalue (Math|Vector|VectorDown)) (Components|Sphere|GetScaledSphereRadius _collision) (Utilities|Array|MakeArray "ObjectTypeQuery1" "ObjectTypeQuery2" "ObjectTypeQuery4") false 0 "None"))
  (if (not _returnvalue_2)
    (Physics|SetPhysicsLinearVelocity (Variables|Default|GetRollingBallMesh) (* (Math|Vector|RotateVectorAroundAxis (Math|Vector|Normalize (+ (Variables|Default|GetDirectionToPlayer) "")) -9e+01 "0, 0,1.000000") (* (Variables|Default|GetInAirMoveForce) (Utilities|Time|GetWorldDeltaSeconds))) true "None")))

(fn UpdateWeaponTransform
  (bind _bazookas (Variables|Default|GetBazookas))
  (bind _collision (Variables|Default|GetCollision))
  (bind _playerref (Variables|Default|GetPlayerRef))
  (bind _playersvelocity (Variables|Default|GetPlayersVelocity))
  (bind _velocityoffset (Variables|Default|GetVelocityOffset))
  (bind _returnvalue (Transformation|GetWorldTransform _collision))
  (bind _returnvalue_2 (Math|Vector|GetForwardVector _collision))
  (bind _output (Utilities|Array|Get(acopy) _bazookas))
  (bind _returnvalue_3 (* _playersvelocity (Math|Vector|MakeVector _velocityoffset _velocityoffset _velocityoffset)))
  (bind _collision_2 (Variables|/Game/Blueprints/BP_Hammond.BP_Hammond_C|GetCollision _playerref))
  (bind _returnvalue_4 (Transformation|GetWorldLocation _collision_2))
  (bind _returnvalue_5 (+ _returnvalue_4 _returnvalue_3))
  (bind _returnvalue_6 (Class|KismetAnimationLibrary|Lookat _returnvalue _returnvalue_5 _returnvalue_2 false "0, 0, 0" 0.0))
  (Transformation|SetWorldRotation (Variables|Default|GetWeaponRingMesh) (Math|Rotator|MakeRotator 0.0 9e+01 (.yaw (.rotation _returnvalue_6))) false false)
  (Transformation|SetActorRelativeRotation _output (Math|Rotator|MakeRotator (.roll (.rotation _returnvalue_6)) (.pitch (.rotation _returnvalue_6)) (.yaw (.rotation _returnvalue_6))))
  (Transformation|SetActorLocation _output (Transformation|GetWorldLocation (Variables|Default|GetWeaponLeft)) false false))

(fn RollBall
  (Class|PrimitiveComponent|SetAllPhysicsAngularVelocityinDegrees (Variables|Default|GetRollingBallMesh) (* (Math|Vector|RotateVectorAroundAxis (Variables|Default|GetDirectionToPlayer) 9e+01 "0, 0,1.000000") (* (Variables|Default|GetRollAcceleration) (/ (Utilities|Time|GetWorldDeltaSeconds) (Variables|Default|GetRollAccelerationTime)))) true)
  (if (> (Math|Vector|VectorLength (Physics|GetPhysicsAngularVelocityinDegrees (Variables|Default|GetRollingBallMesh) "None")) (Variables|Default|GetMaxRollSpeed))
    (Class|PrimitiveComponent|SetAllPhysicsAngularVelocityinDegrees (Variables|Default|GetRollingBallMesh) (* (Variables|Default|GetDirectionToPlayer) (Variables|Default|GetMaxRollSpeed)) false)))